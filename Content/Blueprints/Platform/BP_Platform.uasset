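; Platform actor that switches on material effects matching the effect components attached to it.
; On BeginPlay it creates a dynamic material instance on its StaticMesh, then gathers the EffectName from every BP_AC_PlatformEffect component.
; Each name is used as a scalar parameter name and set to one, so the attached components determine which shader effects show.
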(event `self.ReceiveBeginPlay`
  ; Create shader reference
  (bind _returnvalue (`PrimitiveComponent.CreateDynamicMaterialInstance` (`self.StaticMesh`) 0 null "None"))
  (set `self.Material` _returnvalue)
  ; Read and write data for shader
  (`self.ReadPlatformEffectsNames`)
  (for _array_element (`self.PlatformEffectNames`)
    (`MaterialInstanceDynamic.SetScalarParameterValue` (`self.Material`) _array_element 1.0)))

(fn `ReadPlatformEffectsNames`
  (for _array_element (`self.K2_GetComponentsByClass` "/Game/Blueprints/Platform/BP_AC_PlatformEffect.BP_AC_PlatformEffect_C")
    (`KismetArrayLibrary.Array_Add` (`self.PlatformEffectNames`) (`/Game/Blueprints/Platform/BP_AC_PlatformEffect.EffectName` _array_element))))

(fn `UserConstructionScript`)