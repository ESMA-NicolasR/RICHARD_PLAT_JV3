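; BP_AC_PlatformEffect is an actor component that gives its owning platform hooks for effects on players touching its box.
; It binds to the owner's BoxComponent begin and end overlaps, resolves the third-person character's player controller, and passes it to EffectOnBeginCollision or EffectOnEndCollision.
; Tick polls overlapping characters and calls EffectWhileColliding with their instigator's controller.
; The effect functions are placeholders: begin and end print debug text, while-colliding is empty.
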(event `self.ReceiveBeginPlay`
  (bind _returnvalue (`Actor.GetComponentByClass` (`self.GetOwner`) "/Script/Engine.BoxComponent"))
  (add `PrimitiveComponent.OnComponentBeginOverlap` _returnvalue (delegate `BindBegin`))
  (add `PrimitiveComponent.OnComponentEndOverlap` _returnvalue (delegate `BindEnd`)))

(event `BindBegin`
  (params (OverlappedComponent :type "PrimitiveComponent Object Reference") (OtherActor :type "Actor Object Reference") (OtherComp :type "PrimitiveComponent Object Reference") (OtherBodyIndex :type Integer) (bFromSweep :type Boolean) (SweepResult :type "HitResult Structure (by ref)"))
  (bind _asbp_third_person_character (cast `/Game/Blueprints/Controllers/BP_ThirdPersonCharacter` OtherActor))
  (bind _asbp_my_third_person_player_controller (cast `/Game/Blueprints/Controllers/BP_MyThirdPersonPlayerController` (`Pawn.GetController` _asbp_third_person_character)))
  (`self.EffectOnBeginCollision` _asbp_my_third_person_player_controller))

(event `BindEnd`
  (params (OverlappedComponent :type "PrimitiveComponent Object Reference") (OtherActor :type "Actor Object Reference") (OtherComp :type "PrimitiveComponent Object Reference") (OtherBodyIndex :type Integer))
  (bind _asbp_third_person_character (cast `/Game/Blueprints/Controllers/BP_ThirdPersonCharacter` OtherActor))
  (bind _asbp_my_third_person_player_controller (cast `/Game/Blueprints/Controllers/BP_MyThirdPersonPlayerController` (`Pawn.GetController` _asbp_third_person_character)))
  (`self.EffectOnEndCollision` _asbp_my_third_person_player_controller))

(event `self.ReceiveTick`
  (params (DeltaSeconds :type "Float (single-precision)"))
  (for _array_element (`PrimitiveComponent.GetOverlappingActors` (`Actor.GetComponentByClass` (`self.GetOwner`) "/Script/Engine.BoxComponent") "/Game/Blueprints/Controllers/BP_ThirdPersonCharacter.BP_ThirdPersonCharacter_C")
    (bind _asbp_my_third_person_player_controller (cast `/Game/Blueprints/Controllers/BP_MyThirdPersonPlayerController` (`Pawn.GetController` (`Actor.Instigator` _array_element))))
    (`self.EffectWhileColliding` _asbp_my_third_person_player_controller)))

(fn `EffectOnBeginCollision`
  (params (PlayerController :type "/Game/Blueprints/Controllers/BP_MyThirdPersonPlayerController Object Reference"))
  (`KismetSystemLibrary.PrintString` "BEGIN"))

(fn `EffectOnEndCollision`
  (params (PlayerController :type "/Game/Blueprints/Controllers/BP_MyThirdPersonPlayerController Object Reference"))
  (`KismetSystemLibrary.PrintString` "End"))

(fn `EffectWhileColliding`
  (params (PlayerController :type "/Game/Blueprints/Controllers/BP_MyThirdPersonPlayerController Object Reference")))