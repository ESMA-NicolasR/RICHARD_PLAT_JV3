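; Movement component that carries its owning platform through a series of node actors at a set speed.
; On BeginPlay it teleports the owner to the start node, then each Tick steps toward the current target, clamping movement to avoid overshoot.
; On arrival within a small tolerance it selects the next node, either wrapping around in full-loop mode or reversing direction to ping-pong at the ends.
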(event `self.ReceiveBeginPlay`
  ; Init first target
  (bind _output_get (set `self.CurrentNode` (`self.StartNode`)))
  (bind _output_get_2 (set `self.CurrentTarget` (`Actor.K2_GetActorLocation` (`|GetArrayItem` (`self.Nodes`) _output_get))))
  (`Actor.K2_SetActorLocation` (`self.GetOwner`) _output_get_2 false true))

(event `self.ReceiveTick`
  (params (DeltaSeconds :type "Float (single-precision)"))
  (`self.MoveTowardTarget` DeltaSeconds)
  (bind _returnvalue (`self.CheckHasArrived`))
  (if _returnvalue
    (`self.NextNode`)))

(fn `CheckHasArrived`
  (returns (ReturnValue :type Boolean))
  (return (<= (`KismetMathLibrary.Vector_Distance` (`self.CurrentTarget`) (`Actor.K2_GetActorLocation` (`self.GetOwner`))) 1.0)))

(fn `CheckIsAtTheEnd`
  (returns (IsAtTheEnd :type Boolean))
  (return (== (`self.CurrentNode`) (`KismetMathLibrary.SelectInt` (- (`KismetArrayLibrary.Array_Length` (`self.Nodes`)) 1) 0 (`self.IsForward`)))))

(fn `MoveTowardTarget`
  (params (DeltaSeconds :type "Float (single-precision)"))
  (bind _returnvalue (`self.GetOwner`))
  (bind _returnvalue_2 (`Actor.K2_GetActorLocation` _returnvalue))
  (`Actor.K2_SetActorLocation` _returnvalue (+ (`KismetMathLibrary.ClampVectorSize` (* (`KismetMathLibrary.Normal` (- (`self.CurrentTarget`) (`Actor.K2_GetActorLocation` (`self.GetOwner`)))) (`self.Speed`) DeltaSeconds) 0.0 (`KismetMathLibrary.Vector_Distance` (`self.CurrentTarget`) _returnvalue_2)) _returnvalue_2) false false))

(fn `NextNode`
  (bind _isattheend (`self.CheckIsAtTheEnd`))
  (if _isattheend
    (if (`self.IsFullLoop`)
      (set `self.CurrentNode` (`KismetMathLibrary.SelectInt` 0 (`KismetArrayLibrary.Array_Length` (`self.Nodes`)) (`self.IsForward`)))
      (else
        (set `self.IsForward` (not (`self.IsForward`)))
        (bind _output_get (set `self.CurrentNode` (+ (`self.CurrentNode`) (`KismetMathLibrary.SelectInt` 1 -1 (`self.IsForward`))) :!label _label))))
    (else
      (goto _label)))
  (set `self.CurrentTarget` (`Actor.K2_GetActorLocation` (`|GetArrayItem` (`self.Nodes`) _output_get))))