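; Spiked platform that moves along a straight line between two placed point actors in a repeating loop.
; BeginPlay caches both point locations, scales the timeline play rate by the inverse of LoopTime, then starts it after InitialDelay.
; The timeline's Lerp curve interpolates the actor location without sweep, and the timeline restarts from the start whenever it finishes.
; The graph holds no overlap or damage logic.
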(event `self.ReceiveBeginPlay`
  (`|ExecutionSequence`
    (:`then_0`
      ; Init positions
      (set `self.StartPosition` (`self.K2_GetActorLocation` (`self.StartPoint`)))
      (set `self.EndPosition` (`self.K2_GetActorLocation` (`self.EndPoint`))))
    (:`then_1`
      ; Play movement loop
      (`TimelineComponent.SetPlayRate` (`self.MovementTimeline`) (/ 1.0 (`self.LoopTime`)))
      (`KismetSystemLibrary.Delay` (`self.InitialDelay`))
      (`TimelineComponent.PlayFromStart` (`self.MovementTimeline`)))))

(fn `UserConstructionScript`)