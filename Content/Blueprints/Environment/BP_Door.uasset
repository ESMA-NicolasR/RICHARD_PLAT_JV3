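; BP_Door is a coin-gated door that opens when the player character pays its cost.
; BeginPlay writes the CoinsNeeded price onto CoinNumberText.
; Overlapping the Box asks the third-person controller to spend the coins, then plays either a spend or an error sound.
; On success IsOpen blocks further charges, and the OpenDoor timeline lerps the Door between the ClosePosition and OpenPosition component locations.
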(event `self.ReceiveActorBeginOverlap`
  (params (OtherActor :type "Actor Object Reference")))

(event `self.ReceiveBeginPlay`
  (`TextRenderComponent.K2_SetText` (`self.CoinNumberText`) (`KismetTextLibrary.Conv_StringToText` (`KismetStringLibrary.Concat_StrStr` (`KismetStringLibrary.Conv_IntToString` (`self.CoinsNeeded`)) " coins"))))

(event `self.Box.OnComponentBeginOverlap`
  (params (OverlappedComponent :type "PrimitiveComponent Object Reference") (OtherActor :type "Actor Object Reference") (OtherComp :type "PrimitiveComponent Object Reference") (OtherBodyIndex :type Integer) (bFromSweep :type Boolean) (SweepResult :type "HitResult Structure (by ref)"))
  (cast `/Game/Blueprints/Characters/BP_ThirdPersonCharacter` OtherActor)
  ; Double branch to play sound only if not enough money
  (if (not (`self.IsOpen`))
    (if (`/Game/Blueprints/Controllers/BP_MyThirdPersonPlayerController.SpendCoins` (`/Game/Blueprints/BP_FL_Common.GetMyThirdPersonController`) (`self.CoinsNeeded`))
      (set `self.IsOpen` true)
      (`GameplayStatics.PlaySound2D` "/Game/Audio/A_spend_coin.A_spend_coin" 1.0 1.0 0.0 null null)
      (bind (_direction _lerp) (`Timeline|OpenDoor` :!via `PlayFromStart`)
        (:`Update`
          ; Move down the door
          (`SceneComponent.K2_SetRelativeLocation` (`self.Door`) (`KismetMathLibrary.VLerp` (`SceneComponent.RelativeLocation` (`self.ClosePosition`)) (`SceneComponent.RelativeLocation` (`self.OpenPosition`)) _lerp) false false)))
      (else
        (`GameplayStatics.PlaySound2D` "/Game/Audio/A_error.A_error" 1.0 1.0 0.0 null null)))))

(fn `UserConstructionScript`)