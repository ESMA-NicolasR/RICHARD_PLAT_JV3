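; Base actor component for platform effects that react to the player character touching the owner's Box component.
; On BeginPlay it binds the box's begin and end overlap events, filtering for BP_ThirdPersonCharacter.
; Tick polls the box for overlapping characters to drive a continuous effect.
; Begin, while and end hooks receive the third-person controller and are empty here, apparently for child components to override.
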(event `BindBegin`
  (params (OverlappedComponent :type "PrimitiveComponent Object Reference") (OtherActor :type "Actor Object Reference") (OtherComp :type "PrimitiveComponent Object Reference") (OtherBodyIndex :type Integer) (bFromSweep :type Boolean) (SweepResult :type "HitResult Structure (by ref)"))
  (cast `/Game/Blueprints/Characters/BP_ThirdPersonCharacter` OtherActor)
  (`self.EffectOnBeginCollision` (`/Game/Blueprints/BP_FL_Common.GetMyThirdPersonController`)))

(event `BindEnd`
  (params (OverlappedComponent :type "PrimitiveComponent Object Reference") (OtherActor :type "Actor Object Reference") (OtherComp :type "PrimitiveComponent Object Reference") (OtherBodyIndex :type Integer))
  (cast `/Game/Blueprints/Characters/BP_ThirdPersonCharacter` OtherActor)
  (`self.EffectOnEndCollision` (`/Game/Blueprints/BP_FL_Common.GetMyThirdPersonController`)))

(event `self.ReceiveBeginPlay`
  (add `PrimitiveComponent.OnComponentBeginOverlap` (`Actor.GetComponentByClass` (`self.GetOwner`) "/Script/Engine.BoxComponent") (delegate `BindBegin`))
  (add `PrimitiveComponent.OnComponentEndOverlap` (`Actor.GetComponentByClass` (`self.GetOwner`) "/Script/Engine.BoxComponent") (delegate `BindEnd`)))

(event `self.ReceiveTick`
  (params (DeltaSeconds :type "Float (single-precision)"))
  (for _array_element (`PrimitiveComponent.GetOverlappingActors` (`Actor.GetComponentByClass` (`self.GetOwner`) "/Script/Engine.BoxComponent") "/Game/Blueprints/Characters/BP_ThirdPersonCharacter.BP_ThirdPersonCharacter_C")
    (cast `/Game/Blueprints/Characters/BP_ThirdPersonCharacter` _array_element)
    (`self.EffectWhileColliding` (`/Game/Blueprints/BP_FL_Common.GetMyThirdPersonController`))))

(fn `EffectOnBeginCollision`
  (params (PlayerController :type "/Game/Blueprints/Controllers/BP_MyThirdPersonPlayerController Object Reference")))

(fn `EffectOnEndCollision`
  (params (PlayerController :type "/Game/Blueprints/Controllers/BP_MyThirdPersonPlayerController Object Reference")))

(fn `EffectWhileColliding`
  (params (PlayerController :type "/Game/Blueprints/Controllers/BP_MyThirdPersonPlayerController Object Reference")))